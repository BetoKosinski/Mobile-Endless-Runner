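; BP_RunnerCharacter is the runner character Blueprint; its graph holds only a temporary debug settings menu, marked to move to its own Blueprint later.
; Pressing H creates WBP_SettingsMenu, adds it to the viewport, pauses the game and binds an event to its Quit button.
; The QuitMenu event removes the menu and unpauses the game if the widget is valid.
; The construction script is empty.
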(event `Key|H`
  (params (Key :type "Key Structure"))
  ; Debug Settings Menu (Move to a proper BP Later)
  (:`Pressed`
    (bind _returnvalue (`|CreateWidget` "/Game/Widgets/WBP_SettingsMenu.WBP_SettingsMenu_C"))
    (bind _output_get (set `self.SettingsMenu` _returnvalue))
    (`UserWidget.AddToViewport` _output_get 0)
    (`GameplayStatics.SetGamePaused` true)
    (add `Button.OnClicked` (`/Game/Widgets/WBP_SettingsMenu.QuitButton` (`self.SettingsMenu`)) (`|CreateDelegate` :!event `Quit Menu`))))

(event `Quit Menu`
  ; Debug Settings Menu (Move to a proper BP Later)
  (bind _settingsmenu (`self.SettingsMenu`)
    (:`then`
      (`Widget.RemoveFromParent` _settingsmenu)
      (`GameplayStatics.SetGamePaused` false))
    (:`else`)))

(fn `UserConstructionScript`)